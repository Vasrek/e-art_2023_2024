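; Player character with Enhanced Input look, move and jump, plus checkpoint respawning.
; BeginPlay adds the mapping context and records the starting transform; UpdateCheckpoint replaces it and Death teleports the player back to it.
; Hard-wired test keys fire a debug line trace that re-materials hit BP_TestRaycastCube actors, spawn such cubes nearby, and call a test function on GM_Level1.
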(event Custom|Death
  (Transformation|SetActorTransform (Variables|Default|GetLastCheckpointTransform) false true))

(event Custom|UpdateCheckpoint
  (params (NewCheckpointTransform :type Transform))
  (Variables|Default|SetLastCheckpointTransform NewCheckpointTransform))

(event Input|EnhancedActionEvents|EnhancedInputActionIA_MyLook
  (params (ActionValue :type Vector%202D%20Structure) (ElapsedSeconds :type Float%20%28double-precision%29) (TriggeredSeconds :type Float%20%28double-precision%29) (InputAction :type Input%20Action%20Object%20Reference :default "/Game/Blueprints/Characters/Player/Inputs/Actions/IA_MyLook.IA_MyLook"))
  ;[1 0 0.3756 1 113] Movement
  (Pawn|Input|AddControllerYawInput (.x ActionValue))
  (Pawn|Input|AddControllerPitchInput (.y ActionValue)))

(event Input|EnhancedActionEvents|EnhancedInputActionIA_MyMove
  (params (ActionValue :type Vector%202D%20Structure) (ElapsedSeconds :type Float%20%28double-precision%29) (TriggeredSeconds :type Float%20%28double-precision%29) (InputAction :type Input%20Action%20Object%20Reference :default "/Game/Blueprints/Characters/Player/Inputs/Actions/IA_MyMove.IA_MyMove"))
  ;[1 0 0.3756 1 113] Movement
  (Pawn|Input|AddMovementInput (Math|Vector|GetRightVector (Math|Rotator|MakeRotator 0.0 0.0 (.yaw (Pawn|GetControlRotation :!class /Script/Engine.Pawn)))) (.x ActionValue) false)
  (Pawn|Input|AddMovementInput (Math|Vector|GetForwardVector (Math|Rotator|MakeRotator 0.0 0.0 (.yaw (Pawn|GetControlRotation :!class /Script/Engine.Pawn)))) (.y ActionValue) false))

(event Input|EnhancedActionEvents|EnhancedInputActionIA_MyJump
  (params (ActionValue :type Boolean) (ElapsedSeconds :type Float%20%28double-precision%29) (TriggeredSeconds :type Float%20%28double-precision%29) (InputAction :type Input%20Action%20Object%20Reference :default "/Game/Blueprints/Characters/Player/Inputs/Actions/IA_MyJump.IA_MyJump"))
  ;[1 0 0.3756 1 113] Movement
  (:Started
    (Character|Jump))
  (:Completed
    (Character|StopJumping)))

(event EventBeginPlay
  ;[1 0 0.3756 1 113] Movement
  (bind _asplayer_controller (Utilities|Casting|CastToPlayerController (Pawn|GetController)))
  (Utilities|IsValid (PlayerController|LocalPlayerSubsystems|GetEnhancedInputLocalPlayerSubsystem _asplayer_controller)
    (:Is%20Valid
      (Input|AddMappingContext (PlayerController|LocalPlayerSubsystems|GetEnhancedInputLocalPlayerSubsystem _asplayer_controller) "/Game/Blueprints/Characters/Player/Inputs/IMC_Player.IMC_Player" 0 "(bIgnoreAllPressedKeysUntilRelease=True,bForceImmediately=False,bNotifyUserSettings=False)")
      (Variables|Default|SetLastCheckpointTransform (Transformation|GetActorTransform)))))

(event Input|KeyboardEvents|T
  (params (Key :type Key%20Structure :default "None"))
  (bind _returnvalue (Transformation|GetActorLocation))
  (:Pressed
    (Development|PrintString "Raycast")
    (bind (_outhit _returnvalue_2) (Collision|LineTraceByChannel _returnvalue (+ _returnvalue (* (Math|Vector|GetForwardVector (Pawn|GetControlRotation :!class /Script/Engine.Pawn)) (Variables|Raycast|GetRaycastDistance))) "TraceTypeQuery1" false 0 "ForDuration"))
    (if _returnvalue_2
      (bind _asbp_test_raycast_cube (Utilities|Casting|CastToBP_TestRaycastCube (.HitActor (Collision|BreakHitResult _outhit)))
        (:then
          (Development|PrintString "I have touched raycast cube" true true "(R=0.000000,G=1.000000,B=0.261085,A=1.000000)" 5.0)
          (Rendering|Material|SetMaterial (Variables|/Game/Blueprints/Raycast/BP_TestRaycastCube.BP_TestRaycastCube_C|GetCube _asbp_test_raycast_cube) 0 "/Game/StarterContent/Materials/M_Wood_Oak.M_Wood_Oak"))
        (:CastFailed
          (Development|PrintString "I haven't touched a raycast cube" true true "(R=1.000000,G=0.000000,B=0.181204,A=1.000000)" 5.0))))))

(event Input|KeyboardEvents|J
  (params (Key :type Key%20Structure :default "None"))
  (:Pressed
    (bind _asgm_level_1 (Utilities|Casting|CastToGM_Level1 (Game|GetGameMode)))
    (Default|Test _asgm_level_1)))

(event Input|KeyboardEvents|N
  (params (Key :type Key%20Structure :default "None"))
  (bind _returnvalue (Transformation|GetActorLocation))
  (:Pressed
    (Development|PrintString "Cube Spawner")
    (Game|SpawnActorfromClass "/Game/Blueprints/Raycast/BP_TestRaycastCube.BP_TestRaycastCube_C" (Math|Transform|MakeTransform (Math|Vector|MakeVector (+ (.x _returnvalue) 5e+01) (+ (.y _returnvalue) 5e+01) (+ (.z _returnvalue) 5e+01)) "0, 0, 0" "1.000000,1.000000,1.000000") "Undefined" "MultiplyWithRoot" 0 0)))

(fn ConstructionScript)