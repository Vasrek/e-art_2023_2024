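; Falling platform that shakes when the player character steps into its trigger box, then drops and later respawns.
; A DoOnce-gated overlap plays a timeline that rolls the cube, then enables physics simulation on it when the timeline finishes.
; After a fixed delay, physics is switched off, the cube teleports back to the location cached at BeginPlay, and the DoOnce resets.
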(event OnComponentBeginOverlap(Box)
  (params (OverlappedComponent :type Primitive%20Component%20Object%20Reference) (OtherActor :type Actor%20Object%20Reference) (OtherComp :type Primitive%20Component%20Object%20Reference) (OtherBodyIndex :type Integer) (bFromSweep :type Boolean) (SweepResult :type Hit%20Result%20Structure%20%28by%20ref%29))
  (if (== OtherActor (Game|GetPlayerCharacter 0))
    (Utilities|FlowControl|DoOnce false
      (:Completed
        (CallFunction|ShakingPlatform)))))

(event Custom|ResetFallingDoOnce
  (Utilities|FlowControl|DoOnce false) ; enters at Reset
)

(event Custom|ShakingPlatform
  (bind _rotate (Timeline|ShakingRotation PlayFromStart)
    (:Update
      (Transformation|SetWorldRotation (Variables|Default|GetCube) (Math|Rotator|MakeRotator _rotate 0.0 0.0) false false))
    (:Finished
      (CallFunction|StartFallingPlatform))))

(event Custom|StartFallingPlatform
  (Physics|SetSimulatePhysics (Variables|Default|GetCube) true)
  (Utilities|FlowControl|Delay 5.0)
  (Physics|SetSimulatePhysics (Variables|Default|GetCube) false)
  (Transformation|SetWorldLocationAndRotation (Variables|Default|GetCube) (Variables|Default|GetDefaultLocation) "0, 0, 0" false true)
  (CallFunction|ResetFallingDoOnce))

(event EventBeginPlay
  (Variables|Default|SetDefaultLocation (Transformation|GetWorldLocation (Variables|Default|GetCube))))

(fn ConstructionScript)